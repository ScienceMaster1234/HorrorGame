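; Player character Blueprint with movement, look, jump, sprint and a stamina system, plus an Equip event that swaps the held static mesh.
; Sprinting drains stamina and jumping costs a chunk, while delay-based gain and drain loops re-enter StaminaHandler, which toggles their break flags.
; Near-empty stamina triggers Exhausted, slowing movement and blocking sprint and jump until full recovery restores NormalMovement, which also runs on BeginPlay.
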(event Custom|Equip
  (params (NewMesh :type Static%20Mesh%20Object%20Reference))
  (Components|StaticMesh|SetStaticMesh (Variables|Default|GetEquippedMesh) NewMesh))

(event Custom|DrainStamina
  ;[1 1 1] DrainStamina
  (Variables|Default|SetStamina (Math|Float|Clamp(Float) (- (Variables|Default|GetStamina) 0.5) 0.0 1e+02) :!label _label)
  (CallFunction|StaminaHandler)
  (if (not (Variables|Default|GetDrainStaminaBreak))
    (Utilities|FlowControl|Delay 0.05)
    (goto _label)))

(event Custom|NormalMovement
  (bind _charactermovement (Variables|Character|GetCharacterMovement))
  ;[1 1 1] Normal Movement (Plays on begin)
  (Variables|/Script/Engine.CharacterMovementComponent|SetMaxWalkSpeed _charactermovement 6e+02)
  (Variables|/Script/Engine.CharacterMovementComponent|SetJumpZVelocity _charactermovement 3e+02)
  (Variables|Default|SetIsExhausted false)
  (Variables|Default|SetCanJump%20 true)
  (Variables|Default|SetCanSprint true)
  (Variables|Default|SetIsSprinting false)
  (Variables|Default|SetDrainStaminaBreak false)
  (Variables|Default|SetGainStaminaBreak false))

(event Custom|Exhausted
  ;[1 1 1] Exhaust
  (Variables|/Script/Engine.CharacterMovementComponent|SetMaxWalkSpeed (Variables|Character|GetCharacterMovement) 3e+02)
  (Variables|Default|SetIsSprinting false)
  (Variables|Default|SetCanJump%20 false)
  (Variables|Default|SetCanSprint false)
  (Variables|Default|SetDrainStaminaBreak true)
  (CallFunction|GainStamina))

(event Custom|StaminaHandler
  ;[1 1 1] StaminaHandler
  (Utilities|FlowControl|DelayUntilNextTick)
  (if (Variables|Default|GetIsSprinting)
    (CallFunction|DrainStamina)
    (Variables|Default|SetGainStaminaBreak true)
    (Variables|Default|SetDrainStaminaBreak false)
    (else
      (CallFunction|GainStamina)
      (Variables|Default|SetDrainStaminaBreak true)
      (Variables|Default|SetGainStaminaBreak false)))
  (if (< (Variables|Default|GetStamina) 1.0)
    (CallFunction|Exhausted)
    (elif (== (Variables|Default|GetStamina) 1e+02)
      (CallFunction|NormalMovement))))

(event Custom|GainStamina
  ;[1 1 1] GainStamina
  (Variables|Default|SetStamina (Math|Float|Clamp(Float) (+ (Variables|Default|GetStamina) 0.25) 0.0 1e+02) :!label _label)
  (CallFunction|StaminaHandler)
  (if (not (Variables|Default|GetGainStaminaBreak))
    (Utilities|FlowControl|Delay 0.05)
    (goto _label)))

(event EventBeginPlay
  (CallFunction|NormalMovement)
  (Variables|Default|SetHasBoltCutters false))

(event EventTick
  (params (DeltaSeconds :type Float%20%28single-precision%29)))

(event Input|ActionEvents|InputActionSprint
  (params (Key :type Key%20Structure :default "None"))
  ;[1 1 1] Sprint
  (:Pressed
    (if (Variables|Default|GetCanSprint)
      (Variables|/Script/Engine.CharacterMovementComponent|SetMaxWalkSpeed (Variables|Character|GetCharacterMovement) 1e+03)
      (Variables|Default|SetIsSprinting true)
      (CallFunction|StaminaHandler)))
  (:Released
    (Variables|/Script/Engine.CharacterMovementComponent|SetMaxWalkSpeed (Variables|Character|GetCharacterMovement) 6e+02)
    (Variables|Default|SetIsSprinting false)
    (CallFunction|StaminaHandler)))

(event Input|ActionEvents|InputActionJump
  (params (Key :type Key%20Structure :default "None"))
  (:Pressed
    (if (Variables|Default|GetCanJump%20)
      (Character|Jump)
      (Variables|Default|SetStamina (Math|Float|Clamp(Float) (- (Variables|Default|GetStamina) 15.0) 0.0 1e+02))))
  (:Released
    (Character|StopJumping)))

(event Input|AxisEvents|InputAxisMovementX
  (params (AxisValue :type Float%20%28single-precision%29))
  ;[1 1 1] Walk
  (Pawn|Input|AddMovementInput (Math|Vector|GetRightVector (Math|Rotator|MakeRotator 0.0 0.0 (.Yaw (Math|Rotator|BreakRotator (Pawn|GetControlRotation (Game|GetPlayerController 0) :!class /Script/Engine.Controller))))) AxisValue false))

(event Input|AxisEvents|InputAxisMovementY
  (params (AxisValue :type Float%20%28single-precision%29))
  ;[1 1 1] Walk
  (Pawn|Input|AddMovementInput (Math|Vector|GetForwardVector (Math|Rotator|MakeRotator 0.0 0.0 (.Yaw (Math|Rotator|BreakRotator (Pawn|GetControlRotation (Game|GetPlayerController 0) :!class /Script/Engine.Controller))))) AxisValue false))

(event Input|AxisEvents|InputAxisLookX
  (params (AxisValue :type Float%20%28single-precision%29))
  ;[1 1 1] Look
  (Pawn|Input|AddControllerYawInput AxisValue))

(event Input|AxisEvents|InputAxisLookY
  (params (AxisValue :type Float%20%28single-precision%29))
  ;[1 1 1] Look
  (Pawn|Input|AddControllerPitchInput AxisValue))

(fn ConstructionScript)