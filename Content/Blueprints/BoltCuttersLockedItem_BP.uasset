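; A locked item actor that the player removes by interacting with it while carrying bolt cutters.
; Overlapping its box caches the MyCharacter_BP and enables input on the actor; leaving the box disables it.
; Pressing Interact destroys the actor if the character has bolt cutters, otherwise it shows a HUD widget with a taunting message for two seconds.
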(event OnComponentBeginOverlap(Box)
  (params (OverlappedComponent :type Primitive%20Component%20Object%20Reference) (OtherActor :type Actor%20Object%20Reference) (OtherComp :type Primitive%20Component%20Object%20Reference) (OtherBodyIndex :type Integer) (bFromSweep :type Boolean) (SweepResult :type Hit%20Result%20Structure%20%28by%20ref%29))
  (bind _asmy_character_bp (Utilities|Casting|CastToMyCharacter_BP OtherActor))
  (Input|EnableInput (Game|GetPlayerController 0)))

(event OnComponentEndOverlap(Box)
  (params (OverlappedComponent :type Primitive%20Component%20Object%20Reference) (OtherActor :type Actor%20Object%20Reference) (OtherComp :type Primitive%20Component%20Object%20Reference) (OtherBodyIndex :type Integer))
  (Utilities|Casting|CastToMyCharacter_BP OtherActor)
  (Input|DisableInput (Game|GetPlayerController 0)))

(event Input|ActionEvents|InputActionInteract
  (params (Key :type Key%20Structure :default "None"))
  (:Pressed
    (if (Variables|/Game/Blueprints/MyCharacter_BP.MyCharacter_BP_C|GetHasBoltCutters (stale OnComponentBeginOverlap(Box) _asmy_character_bp))
      (Actor|DestroyActor)
      (else
        (bind _returnvalue (UserInterface|CreateWidget "/Game/Blueprints/HUD.HUD_C" 0 "Maybe You Should Get Some Bitches"))
        (UserInterface|Viewport|AddtoViewport _returnvalue 0)
        (Utilities|FlowControl|Delay 2.0)
        (Widget|RemovefromParent _returnvalue)))))

(fn ConstructionScript)