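; BoltCutters_BP is a bolt cutters pickup that the player collects with the Interact input.
; Its Box overlap enables input for player controller 0 while a MyCharacter_BP is inside and disables it on exit.
; Pressing Interact equips the bolt cutters on the overlapping character, destroys the pickup actor, then sets that character's HasBoltCutters flag.
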(event OnComponentBeginOverlap(Box)
  (params (OverlappedComponent :type Primitive%20Component%20Object%20Reference) (OtherActor :type Actor%20Object%20Reference) (OtherComp :type Primitive%20Component%20Object%20Reference) (OtherBodyIndex :type Integer) (bFromSweep :type Boolean) (SweepResult :type Hit%20Result%20Structure%20%28by%20ref%29))
  (bind _asmy_character_bp (Utilities|Casting|CastToMyCharacter_BP OtherActor))
  (Input|EnableInput (Game|GetPlayerController 0)))

(event OnComponentEndOverlap(Box)
  (params (OverlappedComponent :type Primitive%20Component%20Object%20Reference) (OtherActor :type Actor%20Object%20Reference) (OtherComp :type Primitive%20Component%20Object%20Reference) (OtherBodyIndex :type Integer))
  (Utilities|Casting|CastToMyCharacter_BP OtherActor)
  (Input|DisableInput (Game|GetPlayerController 0)))

(event Input|ActionEvents|InputActionInteract
  (params (Key :type Key%20Structure :default "None"))
  (:Pressed
    (bind _asmy_character_bp (Utilities|Casting|CastToMyCharacter_BP (stale OnComponentBeginOverlap(Box) OtherActor)))
    (Default|Equip _asmy_character_bp "/Game/Assets/BoltCutters.BoltCutters")
    (Actor|DestroyActor)
    (Variables|/Game/Blueprints/MyCharacter_BP.MyCharacter_BP_C|SetHasBoltCutters (stale OnComponentBeginOverlap(Box) _asmy_character_bp) true)))

(fn ConstructionScript)